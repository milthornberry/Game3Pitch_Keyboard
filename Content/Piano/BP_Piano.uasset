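; Walk-on piano actor whose eight keys play notes when the first-person character overlaps them, hosting two puzzles.
; StartAPuzzle uses PuzzleIndex to start either puzzle once, on a piano from BP_PuzzleManager.
; Puzzle 1 lights Hot Cross Buns keys in sequence, using a gate to advance on each correct step until finished.
; Puzzle 2 endlessly lights random keys, flashing green or red by whether the player stands there after a delay.
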(event `self.Key1.OnComponentBeginOverlap`
  (params (OverlappedComponent :type "PrimitiveComponent Object Reference") (OtherActor :type "Actor Object Reference") (OtherComp :type "PrimitiveComponent Object Reference") (OtherBodyIndex :type Integer) (bFromSweep :type Boolean) (SweepResult :type "HitResult Structure (by ref)"))
  ; Play notes on collision with character
  (cast `/Game/FirstPerson/Blueprints/BP_FirstPersonCharacter` OtherActor)
  (`GameplayStatics.SpawnSound2D` "/Game/Piano/Piano1.Piano1" 1.0 1.0 0.0 null)
  (if (not (`self.FinishedPuzzle1`))
    (`self.PlayKey`)))

(event `self.Key5.OnComponentBeginOverlap`
  (params (OverlappedComponent :type "PrimitiveComponent Object Reference") (OtherActor :type "Actor Object Reference") (OtherComp :type "PrimitiveComponent Object Reference") (OtherBodyIndex :type Integer) (bFromSweep :type Boolean) (SweepResult :type "HitResult Structure (by ref)"))
  ; Play notes on collision with character
  (cast `/Game/FirstPerson/Blueprints/BP_FirstPersonCharacter` OtherActor)
  (`GameplayStatics.SpawnSound2D` "/Game/Piano/Piano5.Piano5" 1.0 1.0 0.0 null))

(event `self.Key2.OnComponentBeginOverlap`
  (params (OverlappedComponent :type "PrimitiveComponent Object Reference") (OtherActor :type "Actor Object Reference") (OtherComp :type "PrimitiveComponent Object Reference") (OtherBodyIndex :type Integer) (bFromSweep :type Boolean) (SweepResult :type "HitResult Structure (by ref)"))
  ; Play notes on collision with character
  (cast `/Game/FirstPerson/Blueprints/BP_FirstPersonCharacter` OtherActor)
  (`GameplayStatics.SpawnSound2D` "/Game/Piano/Piano2.Piano2" 1.0 1.0 0.0 null)
  (if (not (`self.FinishedPuzzle1`))
    (`self.PlayKey`)))

(event `self.Key6.OnComponentBeginOverlap`
  (params (OverlappedComponent :type "PrimitiveComponent Object Reference") (OtherActor :type "Actor Object Reference") (OtherComp :type "PrimitiveComponent Object Reference") (OtherBodyIndex :type Integer) (bFromSweep :type Boolean) (SweepResult :type "HitResult Structure (by ref)"))
  ; Play notes on collision with character
  (cast `/Game/FirstPerson/Blueprints/BP_FirstPersonCharacter` OtherActor)
  (`GameplayStatics.SpawnSound2D` "/Game/Piano/Piano6.Piano6" 1.0 1.0 0.0 null))

(event `self.Key3.OnComponentBeginOverlap`
  (params (OverlappedComponent :type "PrimitiveComponent Object Reference") (OtherActor :type "Actor Object Reference") (OtherComp :type "PrimitiveComponent Object Reference") (OtherBodyIndex :type Integer) (bFromSweep :type Boolean) (SweepResult :type "HitResult Structure (by ref)"))
  ; Play notes on collision with character
  (cast `/Game/FirstPerson/Blueprints/BP_FirstPersonCharacter` OtherActor)
  (`GameplayStatics.SpawnSound2D` "/Game/Piano/Piano3.Piano3" 1.0 1.0 0.0 null)
  (if (not (`self.FinishedPuzzle1`))
    (`self.PlayKey`)))

(event `self.Key7.OnComponentBeginOverlap`
  (params (OverlappedComponent :type "PrimitiveComponent Object Reference") (OtherActor :type "Actor Object Reference") (OtherComp :type "PrimitiveComponent Object Reference") (OtherBodyIndex :type Integer) (bFromSweep :type Boolean) (SweepResult :type "HitResult Structure (by ref)"))
  ; Play notes on collision with character
  (cast `/Game/FirstPerson/Blueprints/BP_FirstPersonCharacter` OtherActor)
  (`GameplayStatics.SpawnSound2D` "/Game/Piano/Piano7.Piano7" 1.0 1.0 0.0 null))

(event `self.Key4.OnComponentBeginOverlap`
  (params (OverlappedComponent :type "PrimitiveComponent Object Reference") (OtherActor :type "Actor Object Reference") (OtherComp :type "PrimitiveComponent Object Reference") (OtherBodyIndex :type Integer) (bFromSweep :type Boolean) (SweepResult :type "HitResult Structure (by ref)"))
  ; Play notes on collision with character
  (cast `/Game/FirstPerson/Blueprints/BP_FirstPersonCharacter` OtherActor)
  (`GameplayStatics.SpawnSound2D` "/Game/Piano/Piano4.Piano4" 1.0 1.0 0.0 null))

(event `self.Key8.OnComponentBeginOverlap`
  (params (OverlappedComponent :type "PrimitiveComponent Object Reference") (OtherActor :type "Actor Object Reference") (OtherComp :type "PrimitiveComponent Object Reference") (OtherBodyIndex :type Integer) (bFromSweep :type Boolean) (SweepResult :type "HitResult Structure (by ref)"))
  ; Play notes on collision with character
  (cast `/Game/FirstPerson/Blueprints/BP_FirstPersonCharacter` OtherActor)
  (`GameplayStatics.SpawnSound2D` "/Game/Piano/Piano8.Piano8" 1.0 1.0 0.0 null))

(event `self.ReceiveBeginPlay`
  (bind _key2 (`self.Key2`))
  (bind _key3 (`self.Key3`))
  (bind _key1 (`self.Key1`))
  (bind _returnvalue (`GameplayStatics.GetActorOfClass` "/Game/FirstPerson/Blueprints/BP_FirstPersonCharacter.BP_FirstPersonCharacter_C"))
  (set `self.BPCharacter` _returnvalue)
  (set `self.KeyArray` (`|MakeArray` (`self.Key1`) (`self.Key2`) (`self.Key3`) (`self.Key4`) (`self.Key5`) (`self.Key6`) (`self.Key7`) (`self.Key8`)))
  (bind _returnvalue_2 (`GameplayStatics.GetActorOfClass` "/Game/BP_PuzzleManager.BP_PuzzleManager_C"))
  (set `self.PuzzleManager` _returnvalue_2)
  (set `self.HotCrossBunsArray` (`|MakeArray` _key3 _key2 _key1 _key3 _key2 _key1 _key1 _key1 _key1 _key1 _key2 _key2 _key2 _key2 _key3 _key2 _key1)))

(event `StartAPuzzle`
  (switch `int` (`self.PuzzleIndex`)
    (:`0`
      (if (`self.Puzzle1Started`)
        (`KismetSystemLibrary.PrintString` "You already started puzzle 1")
        (else
          (`self.PlayASong` (`|GetArrayItem` (`/Game/BP_PuzzleManager.PianoArray` (`self.PuzzleManager`))))
          (set `self.Puzzle1Started` true))))
    (:`1`
      (if (`self.Puzzle2Started`)
        (`KismetSystemLibrary.PrintString` "You already started puzzle 2")
        (else
          (`self.EmissiveKeyLoop` (`|GetArrayItem` (`/Game/BP_PuzzleManager.PianoArray` (`self.PuzzleManager`)) 1))
          (set `self.Puzzle2Started` true))))))

(event `PlayKey`
  ; Puzzle 1
  (if (`PrimitiveComponent.IsOverlappingActor` (`self.EmmisiveKey`) (`self.BPCharacter`))
    (`/Engine/EditorBlueprintResources/StandardMacros.Gate` true :!label _label
      (:`Exit`
        (`KismetSystemLibrary.PrintString` "Key Reached" true true (struct :`G` 0.512153 :`B` 0.062463 :`A` 1.0))
        (`PrimitiveComponent.SetMaterial` (stale _output_get) 0 "/AnimationSharing/AnimSharingGreen.AnimSharingGreen")
        (`KismetSystemLibrary.Delay` 0.5)
        (`PrimitiveComponent.SetMaterial` (stale _output_get) 0 "/Engine/BasicShapes/BasicShapeMaterial.BasicShapeMaterial")
        (`KismetSystemLibrary.RetriggerableDelay` 0.0 :!label _label_2)
        (bind _result (`/Engine/EditorBlueprintResources/StandardMacros.IncrementInt` (`self.SongIndex`))
          (:`  `
            (if (== _result 17)
              (`KismetSystemLibrary.PrintString` "You finished the song!")
              (set `self.FinishedPuzzle1` true)
              (else
                (bind _output_get (set `self.EmmisiveKey` (`|GetArrayItem` (`self.HotCrossBunsArray`) (`self.SongIndex`))))
                (`PrimitiveComponent.SetMaterial` _output_get 0 "/Game/M_EmmisiveKey.M_EmmisiveKey")
                (goto _label :!via `Open`)))))))))

(event `PlayASong`
  ; Puzzle 1
  (goto _label_2))

(event `EmissiveKeyLoop`
  ; Puzzle 2
  (`KismetSystemLibrary.RetriggerableDelay` 0.0 :!label _label_3)
  (bind _output_get (set `self.EmmisiveKey` (`|GetArrayItem` (`self.KeyArray`) (`KismetMathLibrary.RandomIntegerInRange` 0 7))))
  (`PrimitiveComponent.SetMaterial` _output_get 0 "/Game/M_EmmisiveKey.M_EmmisiveKey")
  (`KismetSystemLibrary.Delay` 2.0)
  (if (`PrimitiveComponent.IsOverlappingActor` (`self.EmmisiveKey`) (`self.BPCharacter`))
    (`KismetSystemLibrary.PrintString` "Key Reached" true true (struct :`G` 0.512153 :`B` 0.062463 :`A` 1.0))
    (`PrimitiveComponent.SetMaterial` _output_get 0 "/AnimationSharing/AnimSharingGreen.AnimSharingGreen")
    (`KismetSystemLibrary.Delay` 2.0)
    (`PrimitiveComponent.SetMaterial` _output_get 0 "/Engine/BasicShapes/BasicShapeMaterial.BasicShapeMaterial")
    (goto _label_3)
    (else
      (`KismetSystemLibrary.PrintString` "Key Not Reached" true true (struct :`R` 1.0 :`G` 0.11966 :`B` 0.061527 :`A` 1.0))
      (`PrimitiveComponent.SetMaterial` _output_get 0 "/AnimationSharing/AnimSharingRed.AnimSharingRed")
      (`KismetSystemLibrary.Delay` 2.0)
      (`PrimitiveComponent.SetMaterial` _output_get 0 "/Engine/BasicShapes/BasicShapeMaterial.BasicShapeMaterial")
      (goto _label_3))))

(fn `UserConstructionScript`)