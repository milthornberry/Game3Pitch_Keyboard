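; Puzzle manager that starts the piano puzzle matching the trigger the first-person player is standing in.
; On BeginPlay it caches the player character and the BP_Piano actor found in the level.
; StartPuzzle scans the PuzzleTriggers array for the first one overlapping the player, then passes that array index to the piano as PuzzleIndex and calls StartAPuzzle.
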(event `self.ReceiveBeginPlay`
  (bind _returnvalue (`GameplayStatics.GetActorOfClass` "/Game/FirstPerson/Blueprints/BP_FirstPersonCharacter.BP_FirstPersonCharacter_C"))
  (set `self.PlayerCharacter` _returnvalue)
  (bind _returnvalue_2 (`GameplayStatics.GetActorOfClass` "/Game/Piano/BP_Piano.BP_Piano_C"))
  (set `self.BPPiano` _returnvalue_2))

(event `StartPuzzle`
  (bind _bppiano (`self.BPPiano`))
  (for (_array_element _array_index) (`self.PuzzleTriggers`)
    (if (`self.IsOverlappingActor` _array_element (`self.PlayerCharacter`))
      (set `/Game/Piano/BP_Piano.PuzzleIndex` _array_index _bppiano)
      (`/Game/Piano/BP_Piano.StartAPuzzle` _bppiano)
      (break))))

(fn `UserConstructionScript`)